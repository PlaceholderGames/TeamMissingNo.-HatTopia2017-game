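; Train-themed level room actor that dresses itself with rail meshes, random barrels and tumbleweeds, and has removable walls.
; The construction script places static mesh components at even spacing along three rail splines, optionally oriented to them.
; Unless NoSpawn is set, BeginPlay randomly scatters barrels, culling those failing a vertical trace, and the player's first overlap may spawn tumbleweeds.
; DestroyWallFunction removes the east, west or south wall by ID, reporting success.
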(event `self.ReceiveBeginPlay`
  (if (not (`self.NoSpawn`))
    (`ActorComponent.K2_DestroyComponent` (`self.WallOrigin`))
    (`self.GenerateBarrels`)))

(event `self.OverlapCheck.OnComponentBeginOverlap`
  (params (OverlappedComponent :type "PrimitiveComponent Object Reference") (OtherActor :type "Actor Object Reference") (OtherComp :type "PrimitiveComponent Object Reference") (OtherBodyIndex :type Integer) (bFromSweep :type Boolean) (SweepResult :type "HitResult Structure (by ref)"))
  (cast `/Game/TopDownBP/Blueprints/TopDownCharacter` OtherActor)
  (if (not (`self.NoSpawn`))
    (`/Engine/EditorBlueprintResources/StandardMacros.DoOnce` false
      (:`Completed`
        (switch `int` (`KismetMathLibrary.RandomInteger` 3)
          (:`0`
            _)
          (:`1`
            _))
        (for _index (range 4)
          (switch `int` (`KismetMathLibrary.RandomInteger` 3)
            (:`0`
              _)
            (:`1`
              _))
          (`|SpawnActorFromClass` "/Game/Blueprints/BP_TumbleWeed.BP_TumbleWeed_C" (`KismetMathLibrary.MakeTransform` (select `int` _index :`0` (`SceneComponent.K2_GetComponentLocation` (`self.Spawn_2`)) :`1` (`SceneComponent.K2_GetComponentLocation` (`self.Spawn_3`)) :`2` (`SceneComponent.K2_GetComponentLocation` (`self.Spawn_4`)) :`3` (`SceneComponent.K2_GetComponentLocation` (`self.Spawn_1`)))) "Undefined" "OverrideRootScale"))))))

(event `DestroyWall`
  (params (SocketID :type Integer))
  (`ActorComponent.K2_DestroyComponent` (select `int` SocketID :`0` (`self.WallE`) :`1` (`self.WallW`) :`2` (`self.WallS`))))

(event `GenerateBarrels`
  (bind _spawnlocations (`self.SpawnLocations`))
  (bind _returnvalue (`KismetMathLibrary.MakeTransform` (+ (`self.K2_GetActorLocation`) (* (`KismetMathLibrary.GreaterGreater_VectorRotator` (`KismetMathLibrary.MakeVector` (`KismetMathLibrary.RandomFloatInRange` (.x (`|GetArrayItem` _spawnlocations)) (.x (`|GetArrayItem` _spawnlocations 1))) (`KismetMathLibrary.RandomFloatInRange` (.y (`|GetArrayItem` _spawnlocations)) (.y (`|GetArrayItem` _spawnlocations 1)))) (`self.K2_GetActorRotation`)) 0.5))))
  (`KismetSystemLibrary.Delay` (* (`GameplayStatics.GetWorldDeltaSeconds`) 2.0))
  (switch `int` (`KismetMathLibrary.RandomInteger` 3)
    (:`1`
      (for _ (range (+ (`KismetMathLibrary.RandomInteger` 5) 1))
        (bind _returnvalue_2 (`|SpawnActorFromClass` "/Game/Blueprints/BP_Barrel.BP_Barrel_C" _returnvalue "AdjustIfPossibleButDontSpawnIfColliding" "OverrideRootScale"))
        (bind _returnvalue_3 (`self.K2_GetActorLocation` _returnvalue_2))
        (bind (_outhit _returnvalue_4) (`KismetSystemLibrary.LineTraceSingle` (+ _returnvalue_3 (0.0 0.0 1000.0)) (+ _returnvalue_3 (0.0 0.0 -100.0)) "TraceTypeQuery1" false (`|MakeArray` _returnvalue_2 :!type "Actor Object Reference") "None" false))
        (if (not _returnvalue_4)
          (`self.K2_DestroyActor` _returnvalue_2))))
    (:`2`
      (for _ (range (+ (`KismetMathLibrary.RandomIntegerInRange` 3 12) 1))
        (bind _returnvalue_5 (`|SpawnActorFromClass` "/Game/Blueprints/BP_Barrel.BP_Barrel_C" _returnvalue "AdjustIfPossibleButDontSpawnIfColliding" "OverrideRootScale"))
        (bind _returnvalue_6 (`self.K2_GetActorLocation` _returnvalue_5))
        (bind (_outhit_2 _returnvalue_7) (`KismetSystemLibrary.LineTraceSingle` (+ _returnvalue_6 (0.0 0.0 1000.0)) (+ _returnvalue_6 (0.0 0.0 -100.0)) "TraceTypeQuery1" false (`|MakeArray` _returnvalue_5 :!type "Actor Object Reference") "None" false))
        (if (not _returnvalue_7)
          (`self.K2_DestroyActor` _returnvalue_5))))))

(fn `DestroyWallFunction`
  (params (ID :type Integer))
  (returns (Valid :type Boolean))
  (bind _returnvalue (select `int` ID :`0` (`self.WallE`) :`1` (`self.WallW`) :`2` (`self.WallS`)))
  (if (`KismetSystemLibrary.IsValid` _returnvalue)
    (`ActorComponent.K2_DestroyComponent` _returnvalue)
    (return true)
    (else
      (return false))))

(fn `UserConstructionScript`
  (bind _spacing (`self.Spacing`))
  (for _array_element (`|MakeArray` (`self.Rail1`) (`self.Rail2`) (`self.Rail3`))
    (if (> (`self.MeshNumber`) 0)
      (for _index (range (+ (`.ReturnValue` (`KismetMathLibrary.FMod` (`SplineComponent.GetSplineLength` _array_element) _spacing)) 1))
        (bind _returnvalue (* _index _spacing))
        (bind _returnvalue_2 (`AddComponent|NODE_AddStaticMeshComponent-0` :`RelativeTransform` (`KismetMathLibrary.MakeTransform` (`KismetMathLibrary.InverseTransformLocation` (`self.GetTransform`) (`SplineComponent.GetLocationAtDistanceAlongSpline` _array_element _returnvalue "World")) (struct) (1.0 1.0 1.0)))) ; Add static mesh component
        (if (`self.OrientToSpline`)
          (`SceneComponent.K2_SetWorldRotation` _returnvalue_2 (`SplineComponent.GetRotationAtDistanceAlongSpline` _array_element _returnvalue "World") false false) ; Rotate mesh to match direction of spline at its position
        )))))