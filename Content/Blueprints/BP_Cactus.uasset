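; BP_Cactus is a billboard-sprite cactus hazard that damages the player's top-down character and can be chopped by projectiles.
; A TopDownCharacter overlapping its capsule takes one point of damage.
; A BP_Projectile hit swaps the sprite to a chopped version, disables capsule collision and spawns a burst particle effect.
; The chopped cactus stays in the level, as the destroy and emitter-scaling nodes are disconnected.
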(event `self.Capsule.OnComponentBeginOverlap`
  (params (OverlappedComponent :type "PrimitiveComponent Object Reference") (OtherActor :type "Actor Object Reference") (OtherComp :type "PrimitiveComponent Object Reference") (OtherBodyIndex :type Integer) (bFromSweep :type Boolean) (SweepResult :type "HitResult Structure (by ref)"))
  (bind _astop_down_character (cast `/Game/TopDownBP/Blueprints/TopDownCharacter` OtherActor))
  (`/Game/TopDownBP/Blueprints/TopDownCharacter.TakeDamage` _astop_down_character 1))

(event `self.Capsule.OnComponentHit`
  (params (HitComponent :type "PrimitiveComponent Object Reference") (OtherActor :type "Actor Object Reference") (OtherComp :type "PrimitiveComponent Object Reference") (NormalImpulse :type "Vector Structure") (Hit :type "HitResult Structure (by ref)"))
  (cast `/Game/Blueprints/BP_Projectile` OtherActor)
  (`BillboardComponent.SetSprite` (`self.Billboard`) "/Game/Materials/TX_Cactus_01_Chopped.TX_Cactus_01_Chopped")
  (`PrimitiveComponent.SetCollisionEnabled` (`self.Capsule`) "NoCollision")
  (bind _returnvalue (`GameplayStatics.SpawnEmitterAtLocation` "/Game/Effects/P_CactiBurst.P_CactiBurst" (`self.K2_GetActorLocation`))))

(fn `UserConstructionScript`)