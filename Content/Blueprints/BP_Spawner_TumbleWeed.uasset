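; BP_Spawner_TumbleWeed is a spawner actor that periodically spawns BP_TumbleWeed actors at a set of stored locations.
; Tick counts a Timer variable down by world delta seconds.
; When the timer drops below zero, it spawns one tumbleweed at every entry in SpawnLocations with zero rotation and unit scale, then resets to an eight-second interval.
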(event `self.ReceiveTick`
  (params (DeltaSeconds :type "Float (single-precision)"))
  (bind _output_get (set `self.Timer` (- (`self.Timer`) (`GameplayStatics.GetWorldDeltaSeconds`))))
  (if (< _output_get 0.0)
    (for _array_element (`self.SpawnLocations`)
      (`|SpawnActorFromClass` "/Game/Blueprints/BP_TumbleWeed.BP_TumbleWeed_C" (`KismetMathLibrary.MakeTransform` _array_element) "Undefined" "OverrideRootScale"))
    (set `self.Timer` 8.0)))

(fn `UserConstructionScript`)