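; BP_Twister is an enemy that continuously chases the player by reissuing AIMoveTo whenever a move succeeds or fails.
; Projectile hits spawn a hay burst, play a tumbleweed sound and cost a hit point, unless it is spinning.
; Surviving a hit triggers a one-second invulnerable spin with a material swap; death has a one-in-eight chance to drop a random hat pickup.
; Sprite bounce and camera-facing logic is left disconnected.
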(event `ResetMovement`
  (`|AIMoveTo` self (0.0 0.0 0.0) (`GameplayStatics.GetPlayerPawn` 0) :!label _label
    (:`OnSuccess`
      _)
    (:`OnFail`
      _))
  (`self.ResetMovement`))

(event `self.ReceiveBeginPlay`
  (set `self.SpriteStartRotation` (`SceneComponent.RelativeRotation` (`self.PaperSprite`)))
  (set `self.SpriteStartLocation` (`SceneComponent.RelativeLocation` (`self.PaperSprite`)))
  (goto _label))

(event `self.ReceiveTick`
  (params (DeltaSeconds :type "Float (single-precision)")))

(event `self.CapsuleComponent.OnComponentHit`
  (params (HitComponent :type "PrimitiveComponent Object Reference") (OtherActor :type "Actor Object Reference") (OtherComp :type "PrimitiveComponent Object Reference") (NormalImpulse :type "Vector Structure") (Hit :type "HitResult Structure (by ref)"))
  (cast `/Game/Blueprints/BP_Projectile` OtherActor)
  (if (not (`self.spinning`))
    (`GameplayStatics.SpawnEmitterAtLocation` "/Game/Effects/P_HayBurst.P_HayBurst" (`self.K2_GetActorLocation`))
    (`GameplayStatics.PlaySoundAtLocation` "/Game/Sound/CUE_TumbleWeed.CUE_TumbleWeed" (`self.K2_GetActorLocation`))
    (bind _output_get (set `self.HitPoints` (- (`self.HitPoints`) 1)))
    (if (<= _output_get 0)
      (switch `int` (`KismetMathLibrary.RandomInteger` 8)
        (:`0`
          (`|SpawnActorFromClass` "/Game/Blueprints/BP_HatPickup.BP_HatPickup_C" (`KismetMathLibrary.MakeTransform` (`self.K2_GetActorLocation`)) "Undefined" "OverrideRootScale" null (`KismetMathLibrary.RandomInteger` 3))
          (`self.K2_DestroyActor`))
        (:`1`
          (`self.K2_DestroyActor` :!label _label_2))
        (:`2`
          (goto _label_2))
        (:`3`
          (goto _label_2))
        (:`4`
          (goto _label_2))
        (:`5`
          (goto _label_2))
        (:`6`
          (goto _label_2))
        (:`7`
          (goto _label_2))
        (:`8`
          (goto _label_2)))
      (else
        (`self.start spinning`)))))

(event `start spinning`
  (`PrimitiveComponent.SetMaterial` (`self.Sphere`) 0 "/Game/Materials/m_twister1.m_twister1")
  (set `self.spinning` true)
  (`KismetSystemLibrary.Delay` 1.0)
  (set `self.spinning` false)
  (`PrimitiveComponent.SetMaterial` (`self.Sphere`) 0 "/Game/Materials/m_twister.m_twister"))

(fn `UserConstructionScript`)