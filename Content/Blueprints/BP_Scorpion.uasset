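; Sprite-based scorpion enemy that, after first seeing the player, repeatedly repositions around them and fires projectiles.
; It retries while a trace near the player is blocked, then flips its sprite and moves to a random nearby point.
; If in range, a scale Timeline plays forward to shoot and reverses via FlipFlop before moving again.
; Player projectiles reduce its health until destroyed, and touching it damages the player.
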(event `self.ReceiveBeginPlay`)

(event `MoveToFirePosition`
  (bind _returnvalue (`GameplayStatics.GetPlayerPawn` 0))
  (bind _papersprite (`self.PaperSprite`))
  (bind _dangerzoneradius (`self.DangerZoneRadius`))
  (bind _dangerzoneradius_2 (`self.DangerZoneRadius`))
  (bind _returnvalue_2 (`self.K2_GetActorLocation` _returnvalue))
  (bind _returnvalue_3 (`KismetMathLibrary.MakeVector` (+ (.x _returnvalue_2) (`KismetMathLibrary.RandomFloatInRange` (* _dangerzoneradius_2 -1.0) _dangerzoneradius_2)) (+ (.y _returnvalue_2) (`KismetMathLibrary.RandomFloatInRange` (* _dangerzoneradius -1.0) _dangerzoneradius)) (.z _returnvalue_2)))
  (`KismetSystemLibrary.Delay` (`GameplayStatics.GetWorldDeltaSeconds`))
  (bind (_outhit _returnvalue_4) (`KismetSystemLibrary.LineTraceSingle` _returnvalue_3 _returnvalue_2 "TraceTypeQuery1"))
  (if _returnvalue_4
    (`self.MoveToFirePosition`)
    (else
      (if (<= (- (.y (`self.K2_GetActorLocation`)) (.y (`self.K2_GetActorLocation` _returnvalue))) 0.0)
        (`PaperSpriteComponent.SetSprite` _papersprite "/Game/Materials/SPR_Scorpion.SPR_Scorpion")
        (else
          (`PaperSpriteComponent.SetSprite` _papersprite "/Game/Materials/SPR_Scorpion_01.SPR_Scorpion_01")))
      (`|AIMoveTo` self _returnvalue_3
        (:`OnSuccess`
          (`self.FireAtPlayer`))
        (:`OnFail`
          (`self.MoveToFirePosition`))))))

(event `FireAtPlayer`
  (bind _returnvalue (`GameplayStatics.GetPlayerPawn` 0))
  (bind _returnvalue_2 (`self.K2_GetActorLocation`))
  (bind _returnvalue_3 (`KismetMathLibrary.FindLookAtRotation` _returnvalue_2 (`self.K2_GetActorLocation` _returnvalue)))
  (if (<= (`KismetMathLibrary.Abs` (`self.GetDistanceTo` _returnvalue)) 700.0)
    (bind (_direction _scale) (`Timeline|ShootAnimation` :!via `PlayFromStart` :!label _label)
      (:`Update`
        (`SceneComponent.SetRelativeScale3D` (`self.PaperSprite`) (`KismetMathLibrary.MakeVector` 0.3 0.3 _scale)))
      (:`Finished`
        (`/Engine/EditorBlueprintResources/StandardMacros.FlipFlop`
          (:`A`
            (`|SpawnActorFromClass` "/Game/Blueprints/BP_Projectile_Scorpion.BP_Projectile_Scorpion_C" (`KismetMathLibrary.MakeTransform` _returnvalue_2 _returnvalue_3 (`self.ProjectileScale`)) "Undefined" "OverrideRootScale" null (`KismetMathLibrary.GreaterGreater_VectorRotator` (1.0 0.0 0.0) _returnvalue_3))
            (goto _label :!via `ReverseFromEnd`))
          (:`B`
            (`self.MoveToFirePosition` :!label _label_2)
            (`GameplayStatics.PlaySoundAtLocation` "/Game/Sound/SFX_Scorpion.SFX_Scorpion" (`self.K2_GetActorLocation`))))))
    (else
      (goto _label_2))))

(event `self.CapsuleComponent.OnComponentHit`
  (params (HitComponent :type "PrimitiveComponent Object Reference") (OtherActor :type "Actor Object Reference") (OtherComp :type "PrimitiveComponent Object Reference") (NormalImpulse :type "Vector Structure") (Hit :type "HitResult Structure (by ref)"))
  (cast `/Game/Blueprints/BP_Projectile` OtherActor)
  (`GameplayStatics.PlaySoundAtLocation` "/Game/Sound/CUE_Scorpion_Chunk.CUE_Scorpion_Chunk" (`self.K2_GetActorLocation`))
  (bind _output_get (set `self.Health` (- (`self.Health`) 1)))
  (`GameplayStatics.SpawnEmitterAtLocation` "/Game/Effects/P_ScorpionBurst.P_ScorpionBurst" (`self.K2_GetActorLocation`))
  (if (<= _output_get 0)
    (`self.K2_DestroyActor`)))

(event `self.PawnSensing.OnSeePawn`
  (params (Pawn :type "Pawn Object Reference"))
  (cast `/Game/TopDownBP/Blueprints/TopDownCharacter` Pawn)
  (`/Engine/EditorBlueprintResources/StandardMacros.DoOnce` false
    (:`Completed`
      (`self.MoveToFirePosition`)
      (`GameplayStatics.PlaySoundAtLocation` "/Game/Sound/SFX_Scorpion.SFX_Scorpion" (`self.K2_GetActorLocation`)))))

(event `self.CapsuleComponent.OnComponentBeginOverlap`
  (params (OverlappedComponent :type "PrimitiveComponent Object Reference") (OtherActor :type "Actor Object Reference") (OtherComp :type "PrimitiveComponent Object Reference") (OtherBodyIndex :type Integer) (bFromSweep :type Boolean) (SweepResult :type "HitResult Structure (by ref)"))
  (bind _astop_down_character (cast `/Game/TopDownBP/Blueprints/TopDownCharacter` OtherActor))
  (`/Game/TopDownBP/Blueprints/TopDownCharacter.TakeDamage` _astop_down_character 1))

(fn `UserConstructionScript`)