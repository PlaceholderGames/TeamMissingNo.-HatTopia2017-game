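; Saloon door actor with two door components that ease back to their starting rotations whenever they are moved away from them.
; BeginPlay caches both relative rotations in an array and prints the first door's rotation as debug output.
; Tick steers each door toward its cached rotation with RInterpTo, using an exact comparison for the first door and a small tolerance for the second.
; Nothing in these graphs opens the doors.
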(event `self.ReceiveBeginPlay`
  (bind _startrotations (`self.StartRotations`))
  (bind _relativerotation (`SceneComponent.RelativeRotation` (`self.Door`)))
  (`KismetArrayLibrary.Array_Set` _startrotations 0 _relativerotation)
  (`KismetArrayLibrary.Array_Set` _startrotations 1 (`SceneComponent.RelativeRotation` (`self.Door2`)))
  (`KismetSystemLibrary.PrintString` (`KismetStringLibrary.Conv_RotatorToString` _relativerotation)))

(event `self.ReceiveTick`
  (params (DeltaSeconds :type "Float (single-precision)"))
  (bind _output (`|GetArrayItem` (`self.StartRotations`) 1))
  (bind _output_2 (`|GetArrayItem` (`self.StartRotations`)))
  (bind _relativerotation (`SceneComponent.RelativeRotation` (`self.Door2`)))
  (bind _relativerotation_2 (`SceneComponent.RelativeRotation` (`self.Door`)))
  (`|ExecutionSequence`
    (:`then_0`
      (if (not (== _relativerotation_2 _output_2 :`ErrorTolerance` 0.0))
        (`SceneComponent.K2_SetRelativeRotation` (`self.Door`) (`KismetMathLibrary.RInterpTo` _relativerotation_2 _output_2 (`GameplayStatics.GetWorldDeltaSeconds`) 8.0) false false)))
    (:`then_1`
      (if (not (== _relativerotation _output :`ErrorTolerance` 1.0))
        (`SceneComponent.K2_SetRelativeRotation` (`self.Door2`) (`KismetMathLibrary.RInterpTo` _relativerotation _output (`GameplayStatics.GetWorldDeltaSeconds`) 8.0) false false)))))

(fn `UserConstructionScript`)