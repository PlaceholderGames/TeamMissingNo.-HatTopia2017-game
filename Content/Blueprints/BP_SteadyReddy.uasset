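; Boss enemy that stalks the player, fires aimed three-shot bursts and spawns BP_EndLevel when killed.
; Delay-driven event loops cycle LookAtPlayer, AimGun and MoveToNewLocation, using visibility traces and AIMoveTo to random points within DangerZoneRadius of the player.
; While sight holds, a red debug line thickens as a laser telegraph before BP_Projectile_Scorpion shots, then the boss repositions.
; BP_Projectile hits reduce Health and update the player HUD's boss bar.
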(event `AimGun`
  (bind _returnvalue (`GameplayStatics.GetPlayerPawn` 0))
  (bind _returnvalue_2 (`self.K2_GetActorLocation`))
  (bind _returnvalue_3 (`GameplayStatics.GetWorldDeltaSeconds`))
  (bind _speedoverride (`self.SpeedOverride`))
  (bind _ignoreprojectiles (`self.IgnoreProjectiles`))
  (bind _returnvalue_4 (`self.K2_GetActorLocation` _returnvalue))
  (bind _returnvalue_5 (* (`GameplayStatics.GetWorldDeltaSeconds`) 2.0))
  (bind _returnvalue_6 (`KismetMathLibrary.FindLookAtRotation` (`self.K2_GetActorLocation`) (`self.K2_GetActorLocation` (`GameplayStatics.GetPlayerPawn` 0))))
  (bind _returnvalue_7 (`KismetMathLibrary.MakeTransform` (`self.K2_GetActorLocation`) _returnvalue_6 (0.25 0.25 0.25)))
  (bind _returnvalue_8 (`KismetMathLibrary.GreaterGreater_VectorRotator` (1.0 0.0 0.0) _returnvalue_6))
  (`KismetArrayLibrary.Array_Append` _ignoreprojectiles (`|MakeArray` _returnvalue :!type "Actor Object Reference"))
  (bind (_outhit _returnvalue_9) (`KismetSystemLibrary.LineTraceSingle` _returnvalue_2 _returnvalue_4 "TraceTypeQuery1" false _ignoreprojectiles "None" true (struct :`R` 1.0 :`A` 1.0) (struct) _returnvalue_5))
  (`KismetSystemLibrary.DrawDebugLine` _returnvalue_2 _returnvalue_4 (struct :`R` 1.0 :`A` 1.0) _returnvalue_5 (+ (`KismetMathLibrary.Square` (`KismetMathLibrary.Square` (* (- 1.0 (`self.AimTime`)) 2.25))) 1.0))
  (if _returnvalue_9
    (`KismetSystemLibrary.Delay` _returnvalue_3)
    (`self.LookAtPlayer`)
    (else
      (bind _output_get (set `self.AimTime` (- (`self.AimTime`) _returnvalue_3)))
      (if (<= _output_get 0.0)
        (bind _returnvalue_10 (`|SpawnActorFromClass` "/Game/Blueprints/BP_Projectile_Scorpion.BP_Projectile_Scorpion_C" _returnvalue_7 "Undefined" "OverrideRootScale" null _returnvalue_8 _speedoverride))
        (`KismetSystemLibrary.Delay` 0.25)
        (bind _returnvalue_11 (`|SpawnActorFromClass` "/Game/Blueprints/BP_Projectile_Scorpion.BP_Projectile_Scorpion_C" _returnvalue_7 "Undefined" "OverrideRootScale" null _returnvalue_8 _speedoverride))
        (`KismetSystemLibrary.Delay` 0.25)
        (bind _returnvalue_12 (`|SpawnActorFromClass` "/Game/Blueprints/BP_Projectile_Scorpion.BP_Projectile_Scorpion_C" _returnvalue_7 "Undefined" "OverrideRootScale" null _returnvalue_8 _speedoverride))
        (`KismetSystemLibrary.Delay` 1.0)
        (`self.MoveToNewLocation`)
        (else
          (`KismetSystemLibrary.Delay` (`GameplayStatics.GetWorldDeltaSeconds`))
          (`self.AimGun`))))))

(event `LookAtPlayer`
  (bind _returnvalue (`GameplayStatics.GetPlayerPawn` 0))
  (bind _ignoreprojectiles (`self.IgnoreProjectiles`))
  (bind _dangerzoneradius (`self.DangerZoneRadius`))
  (bind _dangerzoneradius_2 (`self.DangerZoneRadius`))
  (bind _returnvalue_2 (`self.K2_GetActorLocation` (`GameplayStatics.GetPlayerPawn` 0)))
  (bind _returnvalue_3 (`KismetMathLibrary.MakeVector` (+ (.x _returnvalue_2) (`KismetMathLibrary.RandomFloatInRange` (* _dangerzoneradius_2 -1.0) _dangerzoneradius_2)) (+ (.y _returnvalue_2) (`KismetMathLibrary.RandomFloatInRange` (* _dangerzoneradius -1.0) _dangerzoneradius)) (.z _returnvalue_2)))
  (bind (_outhit _returnvalue_4) (`KismetSystemLibrary.LineTraceSingle` _returnvalue_3 _returnvalue_2 "TraceTypeQuery1"))
  (if _returnvalue_4
    (`KismetSystemLibrary.Delay` (`GameplayStatics.GetWorldDeltaSeconds`))
    (`self.LookAtPlayer`)
    (else
      (`KismetArrayLibrary.Array_Append` _ignoreprojectiles (`|MakeArray` _returnvalue :!type "Actor Object Reference"))
      (bind (_outhit_2 _returnvalue_5) (`KismetSystemLibrary.LineTraceSingle` (`self.K2_GetActorLocation`) (`self.K2_GetActorLocation` _returnvalue) "TraceTypeQuery1" false _ignoreprojectiles))
      (if _returnvalue_5
        (`|AIMoveTo` self _returnvalue_3
          (:`then`
            (bind (_outhit_3 _returnvalue_6) (`KismetSystemLibrary.LineTraceSingle` :`Start` (`self.K2_GetActorLocation`) :`End` (`self.K2_GetActorLocation` (`GameplayStatics.GetPlayerPawn` 0)) :`TraceChannel` "TraceTypeQuery1" :`TraceColor` (struct :`R` 1.0 :`B` 0.965774 :`A` 1.0) :!label _label))
            (if _returnvalue_6
              (`KismetSystemLibrary.PrintString` "Tis true :'(")
              (`KismetSystemLibrary.Delay` (`GameplayStatics.GetWorldDeltaSeconds`))
              (goto _label)
              (else
                (`MovementComponent.StopMovementImmediately` (`self.CharacterMovement`))
                (`|AIMoveTo` self (`self.K2_GetActorLocation` self) self 1000.0
                  (:`then`
                    (`KismetSystemLibrary.PrintString` "Moving to self"))
                  (:`OnSuccess`
                    (set `self.AimTime` 1.0)
                    (`self.AimGun`))))))
          (:`OnSuccess`
            (`KismetSystemLibrary.Delay` (`GameplayStatics.GetWorldDeltaSeconds`) :!label _label_2)
            (`self.LookAtPlayer`))
          (:`OnFail`
            (goto _label_2)))
        (else
          (set `self.AimTime` 1.0)
          (`self.AimGun`))))))

(event `self.ReceiveBeginPlay`
  (`KismetSystemLibrary.Delay` (`self.AimTime`))
  (`self.LookAtPlayer`)
  (bind _output_get (set `self.BossHealth` (`/Game/UI/W_HUD.BossHealth` (`/Game/TopDownBP/Blueprints/TopDownCharacter.W_HUD` (cast `/Game/TopDownBP/Blueprints/TopDownCharacter` (`GameplayStatics.GetPlayerPawn` 0) :!pure true)))))
  (`Widget.SetVisibility` _output_get "Visible"))

(event `MoveToNewLocation`
  (bind _dangerzoneradius (`self.DangerZoneRadius`))
  (bind _dangerzoneradius_2 (`self.DangerZoneRadius`))
  (bind _returnvalue (`self.K2_GetActorLocation` (`GameplayStatics.GetPlayerPawn` 0)))
  (bind _returnvalue_2 (`KismetMathLibrary.MakeVector` (+ (.x _returnvalue) (`KismetMathLibrary.RandomFloatInRange` (* _dangerzoneradius_2 -1.0) _dangerzoneradius_2)) (+ (.y _returnvalue) (`KismetMathLibrary.RandomFloatInRange` (* _dangerzoneradius -1.0) _dangerzoneradius)) (.z _returnvalue)))
  (bind (_outhit _returnvalue_3) (`KismetSystemLibrary.LineTraceSingle` _returnvalue_2 _returnvalue "TraceTypeQuery1"))
  (if _returnvalue_3
    (`KismetSystemLibrary.Delay` (`GameplayStatics.GetWorldDeltaSeconds`))
    (`self.MoveToNewLocation`)
    (else
      (`|AIMoveTo` self _returnvalue_2
        (:`OnSuccess`
          _)
        (:`OnFail`
          _))
      (`self.LookAtPlayer`))))

(event `self.CapsuleComponent.OnComponentHit`
  (params (HitComponent :type "PrimitiveComponent Object Reference") (OtherActor :type "Actor Object Reference") (OtherComp :type "PrimitiveComponent Object Reference") (NormalImpulse :type "Vector Structure") (Hit :type "HitResult Structure (by ref)"))
  (cast `/Game/Blueprints/BP_Projectile` OtherActor)
  (bind _output_get (set `self.Health` (- (`self.Health`) 1)))
  (`ProgressBar.SetPercent` (`self.BossHealth`) (/ (`KismetMathLibrary.Conv_IntToDouble` _output_get) 200.0))
  (if (<= _output_get 0)
    (`|SpawnActorFromClass` "/Game/Blueprints/BP_EndLevel.BP_EndLevel_C" (`self.GetTransform`) "Undefined" "OverrideRootScale")
    (`self.K2_DestroyActor`)))

(fn `UserConstructionScript`)