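; Procedural level spawner that builds a room layout at BeginPlay, sized by completed levels in GI_HatGame.
; Chains random rectangle, corridor and saloon rooms socket to socket, opening walls and placing BP_EndLevel on the final room.
; Overlaps with other rooms extend the loop; rectangle and saloon collisions branch from a random existing rectangle.
; Rejected rectangles and corridors are destroyed, but the saloon branch destroys the spawner itself; rectangle collisions also add wall plugs.
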(event `self.ReceiveBeginPlay`
  (bind _temprandomint (`self.TempRandomInt`))
  (bind _temprandomint_2 (`self.TempRandomInt`))
  (bind _location (.location (`self.RoomTransform`)))
  (bind _output (`|GetArrayItem` (`self.RoomArray`)))
  (bind _output_2 (`|GetArrayItem` (`self.RoomArray`)))
  (set `self.NumberOfRooms` (* (`/Game/Game/GI_HatGame.LevelsComplete` (cast `/Game/Game/GI_HatGame` (`GameplayStatics.GetGameInstance`) :!pure true)) 6))
  (set `self.RoomTransform` (`KismetMathLibrary.MakeTransform` (`self.K2_GetActorLocation`) (`self.K2_GetActorRotation`) (`self.RoomScale`)))
  (for _index (range (+ (`self.NumberOfRooms`) 1))
    (switch `int` (`KismetMathLibrary.RandomInteger` 7)
      (:`0`
        (bind _returnvalue (== _index 0))
        (bind _returnvalue_2 (`|SpawnActorFromClass` "/Game/Blueprints/BP_Rectangle_4.BP_Rectangle_4_C" (`self.RoomTransform`) "Undefined" "OverrideRootScale" null _returnvalue :!label _label))
        (for _array_element (`PrimitiveComponent.GetOverlappingActors` (`/Game/Blueprints/BP_Rectangle_4.OverlapCheck` _returnvalue_2) null)
          (if (not (== _array_element _returnvalue_2))
            (`/Engine/EditorBlueprintResources/StandardMacros.IsValid` _returnvalue_2
              (:`Is Valid`
                (bind _destroy (`self.CollisionChecker` _array_element))
                (if _destroy
                  ;[1 1 1] Fix wall plug generation
                  (bind _returnvalue_3 (`AddComponent|NODE_AddChildActorComponent-0` :`RelativeTransform` (`KismetMathLibrary.MakeTransform` _location (.rotation (`self.RoomTransform`)) (* (1.0 1.0 1.0) (.x (.scale (`self.RoomTransform`)))))))
                  (`ChildActorComponent.SetChildActorClass` _returnvalue_3 "/Game/Blueprints/BP_WallPlug.BP_WallPlug_C")
                  (`SceneComponent.K2_SetWorldLocation` _returnvalue_3 _location false false)
                  (set `self.NumberOfRooms` (+ (`self.NumberOfRooms`) 1))
                  (bind _outactors (`GameplayStatics.GetAllActorsOfClass` "/Game/Blueprints/BP_Rectangle_4.BP_Rectangle_4_C"))
                  (bind _output_get (set `self.RoomArray` _outactors))
                  (`KismetArrayLibrary.Array_Shuffle` _output_get)
                  (set `self.TempRandomInt` (`KismetMathLibrary.RandomInteger` 3))
                  (set `self.RoomTransform` (`SceneComponent.K2_GetComponentToWorld` (select `int` _temprandomint :`0` (`/Game/Blueprints/BP_Rectangle_4.SocketE` _output) :`1` (`/Game/Blueprints/BP_Rectangle_4.SocketW` _output) :`2` (`/Game/Blueprints/BP_Rectangle_4.SocketS` _output))))
                  (`/Game/Blueprints/BP_Rectangle_4.DestroyWall` _output _temprandomint)
                  (`self.K2_DestroyActor` _returnvalue_2))))))
        (`/Engine/EditorBlueprintResources/StandardMacros.IsValid` _returnvalue_2
          (:`Is Valid`
            (set `self.TempRandomInt` (`KismetMathLibrary.RandomInteger` 3))
            (bind _output_get_2 (set `self.SocketTemp` (select `int` (`self.TempRandomInt`) :`0` (`/Game/Blueprints/BP_Rectangle_4.SocketE` _returnvalue_2) :`1` (`/Game/Blueprints/BP_Rectangle_4.SocketW` _returnvalue_2) :`2` (`/Game/Blueprints/BP_Rectangle_4.SocketS` _returnvalue_2))))
            (if (== _index (`self.NumberOfRooms`))
              (`|SpawnActorFromClass` "/Game/Blueprints/BP_EndLevel.BP_EndLevel_C" (`SceneComponent.K2_GetComponentToWorld` (`/Game/Blueprints/BP_Rectangle_4.Socket_End` _returnvalue_2)) "Undefined" "OverrideRootScale")
              (else
                (`/Game/Blueprints/BP_Rectangle_4.DestroyWall` _returnvalue_2 (`self.TempRandomInt`))))
            (set `self.RoomTransform` (`SceneComponent.K2_GetComponentToWorld` _output_get_2)))))
      (:`1`
        (bind _returnvalue_4 (`|SpawnActorFromClass` "/Game/Blueprints/BP_Corridor_2.BP_Corridor_2_C" (`self.RoomTransform`) "Undefined" "OverrideRootScale" null _returnvalue :!label _label_2))
        (for _array_element_2 (`PrimitiveComponent.GetOverlappingActors` (`/Game/Blueprints/BP_Corridor_2.OverlapCheck` _returnvalue_4) null)
          (if (not (== _array_element_2 _returnvalue_4))
            (`/Engine/EditorBlueprintResources/StandardMacros.IsValid` _returnvalue_4
              (:`Is Valid`
                (bind _destroy_2 (`self.CollisionChecker` _array_element_2))
                (if _destroy_2
                  (set `self.NumberOfRooms` (+ (`self.NumberOfRooms`) 1))
                  (`self.K2_DestroyActor` _returnvalue_4))))))
        (`/Engine/EditorBlueprintResources/StandardMacros.IsValid` _returnvalue_4
          (:`Is Valid`
            (if (== _index (`self.NumberOfRooms`))
              (`|SpawnActorFromClass` "/Game/Blueprints/BP_EndLevel.BP_EndLevel_C" (`SceneComponent.K2_GetComponentToWorld` (`/Game/Blueprints/BP_Corridor_2.Socket_End` _returnvalue_4)) "Undefined" "OverrideRootScale")
              (else
                (`/Game/Blueprints/BP_Corridor_2.DestroyWall` _returnvalue_4)))
            (set `self.RoomTransform` (`SceneComponent.K2_GetComponentToWorld` (`/Game/Blueprints/BP_Corridor_2.SocketS` _returnvalue_4))))))
      (:`2`
        (goto _label))
      (:`3`
        (goto _label))
      (:`4`
        (goto _label_2))
      (:`5`
        (goto _label_2))
      (:`6`
        (bind _returnvalue_5 (`|SpawnActorFromClass` "/Game/Blueprints/BP_Saloon_01.BP_Saloon_01_C" (`self.RoomTransform`) "Undefined" "OverrideRootScale" null _returnvalue))
        (for _array_element_3 (`PrimitiveComponent.GetOverlappingActors` (`/Game/Blueprints/BP_Saloon_01.OverlapCheck` _returnvalue_5) null)
          (if (not (== _array_element_3 _returnvalue_5))
            (`/Engine/EditorBlueprintResources/StandardMacros.IsValid` _returnvalue_5
              (:`Is Valid`
                (bind _destroy_3 (`self.CollisionChecker` _array_element_3))
                (if _destroy_3
                  (set `self.NumberOfRooms` (+ (`self.NumberOfRooms`) 1))
                  (bind _outactors_2 (`GameplayStatics.GetAllActorsOfClass` "/Game/Blueprints/BP_Rectangle_4.BP_Rectangle_4_C"))
                  (bind _output_get_3 (set `self.RoomArray` _outactors_2))
                  (`KismetArrayLibrary.Array_Shuffle` _output_get_3)
                  (set `self.TempRandomInt` (`KismetMathLibrary.RandomInteger` 3))
                  (set `self.RoomTransform` (`SceneComponent.K2_GetComponentToWorld` (select `int` _temprandomint_2 :`0` (`/Game/Blueprints/BP_Rectangle_4.SocketE` _output_2) :`1` (`/Game/Blueprints/BP_Rectangle_4.SocketW` _output_2) :`2` (`/Game/Blueprints/BP_Rectangle_4.SocketS` _output_2))))
                  (`/Game/Blueprints/BP_Rectangle_4.DestroyWall` _output_2 _temprandomint_2)
                  (`self.K2_DestroyActor`))))))
        (`/Engine/EditorBlueprintResources/StandardMacros.IsValid` _returnvalue_5
          (:`Is Valid`
            (set `self.TempRandomInt` (`KismetMathLibrary.RandomInteger` 3))
            (bind _output_get_4 (set `self.SocketTemp` (select `int` (`self.TempRandomInt`) :`0` (`/Game/Blueprints/BP_Saloon_01.SocketE` _returnvalue_5) :`1` (`/Game/Blueprints/BP_Saloon_01.SocketW` _returnvalue_5) :`2` (`/Game/Blueprints/BP_Saloon_01.SocketS` _returnvalue_5))))
            (if (== _index (`self.NumberOfRooms`))
              (`|SpawnActorFromClass` "/Game/Blueprints/BP_EndLevel.BP_EndLevel_C" (`SceneComponent.K2_GetComponentToWorld` (`/Game/Blueprints/BP_Saloon_01.Socket_End` _returnvalue_5)) "Undefined" "OverrideRootScale")
              (else
                (`/Game/Blueprints/BP_Saloon_01.DestroyWall` _returnvalue_5 (`self.TempRandomInt`))
                (set `self.RoomTransform` (`SceneComponent.K2_GetComponentToWorld` _output_get_4))))))))))

(fn `CollisionChecker`
  (params (Actor :type "Actor Object Reference"))
  (returns (Destroy :type Boolean))
  (cast `/Game/Blueprints/BP_Rectangle_4` Actor
    (:`then`
      _)
    (:`CastFailed`
      (cast `/Game/Blueprints/BP_Corridor_2` Actor
        (:`then`
          _)
        (:`CastFailed`
          (cast `/Game/Blueprints/BP_Saloon_01` Actor
            (:`then`
              _)
            (:`CastFailed`
              (return false)))))))
  (return true))

(fn `UserConstructionScript`)