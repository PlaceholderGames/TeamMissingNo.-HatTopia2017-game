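; A destructible barrel actor that shatters when hit by a BP_Projectile or BP_Projectile_Scorpion.
; One frame after BeginPlay, it destroys any other barrels overlapping its Sphere.
; On a qualifying hit, it adds a destructible component at the barrel's transform, breaks it with radius damage and destroys the original Barrel component.
; SetScalePieces then re-calls itself through per-frame Delays, lerping the pieces down to about quarter scale.
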(event `RemoveOverlappingBarrels`
  (`KismetSystemLibrary.Delay` (`GameplayStatics.GetWorldDeltaSeconds`))
  (for _array_element (`PrimitiveComponent.GetOverlappingActors` (`self.Sphere`) "BP_Barrel_C")
    (if (not (== _array_element self))
      (`self.K2_DestroyActor` _array_element))))

(event `self.ReceiveBeginPlay`
  (`self.RemoveOverlappingBarrels`))

(event `self.ReceiveTick`
  (params (DeltaSeconds :type "Float (single-precision)")))

(event `self.Barrel.OnComponentHit`
  (params (HitComponent :type "PrimitiveComponent Object Reference") (OtherActor :type "Actor Object Reference") (OtherComp :type "PrimitiveComponent Object Reference") (NormalImpulse :type "Vector Structure") (Hit :type "HitResult Structure (by ref)"))
  (bind _barrel (`self.Barrel`))
  (cast `/Game/Blueprints/BP_Projectile` OtherActor
    (:`then`
      _)
    (:`CastFailed`
      (cast `/Game/Blueprints/BP_Projectile_Scorpion` OtherActor)))
  (bind _returnvalue (`AddComponent|NODE_AddDestructibleComponent-0` :`RelativeTransform` (`SceneComponent.GetRelativeTransform` _barrel)))
  (`DestructibleComponent.ApplyRadiusDamage` _returnvalue 10000.0 (`self.K2_GetActorLocation`) 0.0 2500.0 false)
  (`ActorComponent.K2_DestroyComponent` _barrel)
  (`self.SetScalePieces`))

(event `SetScalePieces`
  (bind _returnvalue (`KismetMathLibrary.Lerp` (.x (`SceneComponent.K2_GetComponentScale` (stale `self.Barrel.OnComponentHit` _returnvalue))) 0.25 (* (`GameplayStatics.GetWorldDeltaSeconds`) 4.0)))
  (`SceneComponent.SetWorldScale3D` (stale `self.Barrel.OnComponentHit` _returnvalue) (`KismetMathLibrary.MakeVector` _returnvalue _returnvalue _returnvalue))
  (if (not (<= _returnvalue 0.26))
    (`KismetSystemLibrary.Delay` (`GameplayStatics.GetWorldDeltaSeconds`))
    (`self.SetScalePieces`)))

(fn `UserConstructionScript`)