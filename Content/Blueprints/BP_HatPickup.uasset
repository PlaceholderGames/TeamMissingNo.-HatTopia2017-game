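; BP_HatPickup is a hat pickup actor whose appearance is chosen by its HatID.
; The construction script switches on HatID, either enlarging the default Hat sprite or swapping it to a flipped Trilby or Tricorn sprite.
; The event graph has no active logic, so no collection behavior lives here, and leftover sprite and scaling nodes in both graphs are disconnected.
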(event `self.ReceiveBeginPlay`)

(fn `UserConstructionScript`
  (bind _hat (`self.Hat`))
  (switch `int` (`self.HatID`)
    (:`0`
      (`SceneComponent.SetWorldScale3D` _hat (* (`SceneComponent.RelativeScale3D` _hat) 1.67)))
    (:`1`
      (`BillboardComponent.SetSprite` (`self.Hat`) "/Game/Materials/trilby_flipped.trilby_flipped"))
    (:`2`
      (`BillboardComponent.SetSprite` (`self.Hat`) "/Game/Materials/tricorn_flipped.tricorn_flipped"))))