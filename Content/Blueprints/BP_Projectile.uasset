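; BP_Projectile is a projectile actor that destroys itself when its sphere hits anything.
; On BeginPlay it finds the first BP_SteadyReddy and overwrites that actor's IgnoreProjectiles list with every current BP_Projectile.
; On hit it removes itself from that list before destruction.
; Disconnected leftover nodes hold a TopDownCharacter hit check, a debug print and a velocity setter.
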(event `self.ReceiveBeginPlay`
  (bind _outactors (`GameplayStatics.GetAllActorsOfClass` "/Game/Blueprints/BP_SteadyReddy.BP_SteadyReddy_C"))
  (bind _output_get (set `self.SteadyReddy` (`|GetArrayItem` _outactors)))
  (bind _outactors_2 (`GameplayStatics.GetAllActorsOfClass` "BP_Projectile_C"))
  (set `/Game/Blueprints/BP_SteadyReddy.IgnoreProjectiles` _outactors_2 _output_get))

(event `self.Sphere.OnComponentHit`
  (params (HitComponent :type "PrimitiveComponent Object Reference") (OtherActor :type "Actor Object Reference") (OtherComp :type "PrimitiveComponent Object Reference") (NormalImpulse :type "Vector Structure") (Hit :type "HitResult Structure (by ref)"))
  (`KismetArrayLibrary.Array_RemoveItem` (`/Game/Blueprints/BP_SteadyReddy.IgnoreProjectiles` (`self.SteadyReddy`)) self)
  (`self.K2_DestroyActor`))

(fn `UserConstructionScript`)