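; Scorpion boss that chases the player, deals contact damage, spawns BP_Scorpion minions and shows its health on the HUD.
; Once it sees the player, it loops between moving to random nearby points (re-rolled after the visibility trace) and spawning when in range.
; A FlipFlop on the squash timeline's Finished pin alternates spawning and repositioning.
; Projectile hits lower health, raising minion count at thresholds; death sometimes drops a hat.
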(event `self.ReceiveBeginPlay`
  (`KismetSystemLibrary.Delay` 2.0)
  (bind _output_get (set `self.BossHealth` (`/Game/UI/W_HUD.BossHealth` (`/Game/TopDownBP/Blueprints/TopDownCharacter.W_HUD` (cast `/Game/TopDownBP/Blueprints/TopDownCharacter` (`GameplayStatics.GetPlayerPawn` 0) :!pure true)))))
  (`Widget.SetVisibility` _output_get "Visible"))

(event `MoveToFirePosition`
  (bind _returnvalue (`GameplayStatics.GetPlayerPawn` 0))
  (bind _papersprite (`self.PaperSprite`))
  (bind _anim_scorpion (`self.Anim_Scorpion`))
  (bind _dangerzoneradius (`self.DangerZoneRadius`))
  (bind _dangerzoneradius_2 (`self.DangerZoneRadius`))
  (bind _returnvalue_2 (`self.K2_GetActorLocation` _returnvalue))
  (bind _returnvalue_3 (`KismetMathLibrary.MakeVector` (+ (.x _returnvalue_2) (`KismetMathLibrary.RandomFloatInRange` (* _dangerzoneradius_2 -1.0) _dangerzoneradius_2)) (+ (.y _returnvalue_2) (`KismetMathLibrary.RandomFloatInRange` (* _dangerzoneradius -1.0) _dangerzoneradius)) (.z _returnvalue_2)))
  (`KismetSystemLibrary.Delay` (`GameplayStatics.GetWorldDeltaSeconds`))
  (bind (_outhit _returnvalue_4) (`KismetSystemLibrary.LineTraceSingle` _returnvalue_3 _returnvalue_2 "TraceTypeQuery1"))
  (if _returnvalue_4
    (`self.MoveToFirePosition`)
    (`KismetSystemLibrary.PrintString` "Could not find location")
    (else
      (if (<= (- (.y (`self.K2_GetActorLocation`)) (.y (`self.K2_GetActorLocation` _returnvalue))) 0.0)
        (`PaperSpriteComponent.SetSprite` _papersprite "/Game/Materials/SPR_Scorpion.SPR_Scorpion")
        (`SceneComponent.K2_SetRelativeRotation` _anim_scorpion (struct :`Yaw` 90.0 :`Roll` -20.0) false false)
        (else
          (`PaperSpriteComponent.SetSprite` _papersprite "/Game/Materials/SPR_Scorpion_01.SPR_Scorpion_01")
          (`SceneComponent.K2_SetRelativeRotation` _anim_scorpion (struct :`Yaw` -90.0 :`Roll` 20.0) false false)))
      (`|AIMoveTo` self _returnvalue_3
        (:`OnSuccess`
          (`self.FireAtPlayer`))
        (:`OnFail`
          (`self.MoveToFirePosition`))))))

(event `FireAtPlayer`
  (if (<= (`KismetMathLibrary.Abs` (`self.GetDistanceTo` (`GameplayStatics.GetPlayerPawn` 0))) 700.0)
    (bind (_direction _scale) (`Timeline|ShootAnimation` :!via `PlayFromStart` :!label _label)
      (:`Update`
        (`SceneComponent.SetRelativeScale3D` (`self.PaperSprite`) (`KismetMathLibrary.MakeVector` 0.3 0.3 _scale)))
      (:`Finished`
        (`/Engine/EditorBlueprintResources/StandardMacros.FlipFlop`
          (:`A`
            (for _ (range 1 (+ (`self.SpawnNumber`) 1))
              (`|SpawnActorFromClass` "/Game/Blueprints/BP_Scorpion.BP_Scorpion_C" (`KismetMathLibrary.MakeTransform` (.location (`self.GetTransform`)) (.rotation (`self.GetTransform`))) "AdjustIfPossibleButAlwaysSpawn" "OverrideRootScale" null true)
              (goto _label :!via `ReverseFromEnd`))
            (goto _label :!via `ReverseFromEnd`))
          (:`B`
            (`self.MoveToFirePosition` :!label _label_2)
            (`GameplayStatics.PlaySoundAtLocation` "/Game/Sound/SFX_Scorpion.SFX_Scorpion" (`self.K2_GetActorLocation`))))))
    (else
      (goto _label_2))))

(event `self.CapsuleComponent.OnComponentHit`
  (params (HitComponent :type "PrimitiveComponent Object Reference") (OtherActor :type "Actor Object Reference") (OtherComp :type "PrimitiveComponent Object Reference") (NormalImpulse :type "Vector Structure") (Hit :type "HitResult Structure (by ref)"))
  (cast `/Game/Blueprints/BP_Projectile` OtherActor)
  (`GameplayStatics.PlaySoundAtLocation` "/Game/Sound/CUE_Scorpion_Chunk.CUE_Scorpion_Chunk" (`self.K2_GetActorLocation`))
  (bind _output_get (set `self.Health` (- (`self.Health`) 1)))
  (`GameplayStatics.SpawnEmitterAtLocation` "/Game/Effects/P_ScorpionBurst.P_ScorpionBurst" (`self.K2_GetActorLocation`))
  (`ProgressBar.SetPercent` (`self.BossHealth`) (/ (`KismetMathLibrary.Conv_IntToDouble` _output_get) 150.0))
  (if (<= _output_get 0)
    (switch `int` (`KismetMathLibrary.RandomInteger` 8)
      (:`0`
        (`|SpawnActorFromClass` "/Game/Blueprints/BP_HatPickup.BP_HatPickup_C" (`KismetMathLibrary.MakeTransform` (`self.K2_GetActorLocation`)) "Undefined" "OverrideRootScale" null (`KismetMathLibrary.RandomInteger` 5) :!label _label_3)
        (`self.K2_DestroyActor`))
      (:`1`
        (goto _label_3))
      (:`2`
        (`self.K2_DestroyActor` :!label _label_4))
      (:`3`
        (goto _label_4))
      (:`4`
        (goto _label_4))
      (:`5`
        (goto _label_4))
      (:`6`
        (goto _label_4))
      (:`7`
        (goto _label_4))
      (:`8`
        (goto _label_4)))
    (else
      (switch `string` (`KismetStringLibrary.Conv_IntToString` _output_get)
        (:`100`
          (set `self.SpawnNumber` 2))
        (:`50`
          (set `self.SpawnNumber` 3))))))

(event `self.PawnSensing.OnSeePawn`
  (params (Pawn :type "Pawn Object Reference"))
  (cast `/Game/TopDownBP/Blueprints/TopDownCharacter` Pawn)
  (`/Engine/EditorBlueprintResources/StandardMacros.DoOnce` false
    (:`Completed`
      (`self.MoveToFirePosition`)
      (`GameplayStatics.PlaySoundAtLocation` "/Game/Sound/SFX_Scorpion.SFX_Scorpion" (`self.K2_GetActorLocation`)))))

(event `self.CapsuleComponent.OnComponentBeginOverlap`
  (params (OverlappedComponent :type "PrimitiveComponent Object Reference") (OtherActor :type "Actor Object Reference") (OtherComp :type "PrimitiveComponent Object Reference") (OtherBodyIndex :type Integer) (bFromSweep :type Boolean) (SweepResult :type "HitResult Structure (by ref)"))
  (bind _astop_down_character (cast `/Game/TopDownBP/Blueprints/TopDownCharacter` OtherActor))
  (`/Game/TopDownBP/Blueprints/TopDownCharacter.TakeDamage` _astop_down_character 1))

(fn `UserConstructionScript`)