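; Saloon level piece with removable walls that spawns tumbleweeds when the player's TopDownCharacter first enters its OverlapCheck volume.
; Unless NoSpawn is set, BeginPlay removes WallOrigin, and the one-time overlap randomly spawns tumbleweeds at up to three spawn points.
; DestroyWall removes the east, west or south wall by socket ID.
; GenerateBarrels is empty; the random barrel scatter and NoSpawn overlap check are disconnected.
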(event `self.ReceiveBeginPlay`
  (if (not (`self.NoSpawn`))
    (`ActorComponent.K2_DestroyComponent` (`self.WallOrigin`))
    (`self.GenerateBarrels`)))

(event `self.OverlapCheck.OnComponentBeginOverlap`
  (params (OverlappedComponent :type "PrimitiveComponent Object Reference") (OtherActor :type "Actor Object Reference") (OtherComp :type "PrimitiveComponent Object Reference") (OtherBodyIndex :type Integer) (bFromSweep :type Boolean) (SweepResult :type "HitResult Structure (by ref)"))
  (cast `/Game/TopDownBP/Blueprints/TopDownCharacter` OtherActor)
  (if (not (`self.NoSpawn`))
    (`/Engine/EditorBlueprintResources/StandardMacros.DoOnce` false
      (:`Completed`
        (switch `int` (`KismetMathLibrary.RandomInteger` 3)
          (:`0`
            _)
          (:`1`
            _))
        (for _index (range 4)
          (switch `int` (`KismetMathLibrary.RandomInteger` 3)
            (:`0`
              _)
            (:`1`
              _))
          (`|SpawnActorFromClass` "/Game/Blueprints/BP_TumbleWeed.BP_TumbleWeed_C" (`KismetMathLibrary.MakeTransform` (select `int` _index :`0` (`SceneComponent.K2_GetComponentLocation` (`self.Spawn_2`)) :`1` (`SceneComponent.K2_GetComponentLocation` (`self.Spawn_3`)) :`2` (`SceneComponent.K2_GetComponentLocation` (`self.Spawn_1`)))) "Undefined" "OverrideRootScale"))))))

(event `DestroyWall`
  (params (SocketID :type Integer))
  (`ActorComponent.K2_DestroyComponent` (select `int` SocketID :`0` (`self.WallE`) :`1` (`self.WallW`) :`2` (`self.WallS`))))

(event `GenerateBarrels`)

(fn `UserConstructionScript`)